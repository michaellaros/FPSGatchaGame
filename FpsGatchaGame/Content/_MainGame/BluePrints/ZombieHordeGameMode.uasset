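; Game mode for a zombie horde game that spawns a wave of zombies when play begins.
; BeginPlay calls StartGame, which runs SpawnZombies to size the horde from CurrentWave and store it in ZombieTotal and ZombieLeft.
; Two loops spawn BP_Zombie actors, half at each of two spawn transforms, with the first loop breaking at the halfway index.
; The graph contains no wave advancement or kill tracking.
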(event `self.ReceiveBeginPlay`
  (`self.StartGame`))

(event `StartGame`
  (`self.SpawnZombies`))

(event `SpawnZombies`
  (bind _output_get (set `self.ZombieTotal` (* (`self.CurrentWave`) 4)))
  (set `self.ZombieLeft` _output_get)
  (for _index (range (+ _output_get 1))
    (if (== _index (/ (`self.ZombieTotal`) 2))
      (break)
      (else
        (`|SpawnActorFromClass` "/Game/_MainGame/Zombie/BP_Zombie.BP_Zombie_C" (`self.Spawn Location1`) "Undefined" "OverrideRootScale" null null))))
  (for _ (range 1 (+ (/ (`self.ZombieTotal`) 2) 1))
    (`|SpawnActorFromClass` "/Game/_MainGame/Zombie/BP_Zombie.BP_Zombie_C" (`self.Spawn Location2`) "Undefined" "OverrideRootScale" null null)))

(fn `UserConstructionScript`)