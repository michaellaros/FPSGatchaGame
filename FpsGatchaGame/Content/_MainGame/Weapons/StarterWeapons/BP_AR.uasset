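; BP_AR is a starter assault rifle that attaches to the first-person character's mesh on overlap and binds to its use-item event.
; Each shot checks ammo and reload state, plays an aim or idle fire montage, then line-traces from the camera.
; Physical surface types separate head and body hits for point damage, with a "Zombie" tag fallback.
; Hits spawn blood or asphalt particles, and traces leave persistent debug lines.
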(event `self.SphereCollision.OnComponentBeginOverlap`
  (params (OverlappedComponent :type "PrimitiveComponent Object Reference") (OtherActor :type "Actor Object Reference") (OtherComp :type "PrimitiveComponent Object Reference") (OtherBodyIndex :type Integer) (bFromSweep :type Boolean) (SweepResult :type "HitResult Structure (by ref)"))
  (bind _asbp_first_person_character (cast `/Game/_MainGame/BluePrints/BP_FirstPersonCharacter` OtherActor)
    (:`then`
      (bind _output_get (set `self.As BP First Person Character` _asbp_first_person_character))
      (`self.K2_AttachToComponent` self (`/Game/_MainGame/BluePrints/BP_FirstPersonCharacter.FirstPersonMesh` _output_get) "ArPoint" "SnapToTarget" "SnapToTarget" "SnapToTarget" true)
      (add `/Game/_MainGame/BluePrints/BP_FirstPersonCharacter.OnUseItem` (`self.As BP First Person Character`) (`|CreateDelegate` :!event `ShootEvent`)))
    (:`CastFailed`
      (`KismetSystemLibrary.PrintString` "Cast to BP_FirstPersonCharacter FAILED"))))

(event `ShootEvent`
  (bind _returnvalue (`GameplayStatics.GetPlayerCameraManager` 0))
  (bind _returnvalue_2 (`PlayerCameraManager.GetCameraLocation` _returnvalue))
  (if (> (`self.Magazine_0_0`) 0)
    (if (not (`self.isReloading_0`))
      (`/Engine/EditorBlueprintResources/StandardMacros.DecrementInt` (`self.Magazine_0_0`)
        (:`  `
          (bind _asbp_first_person_character (cast `/Game/_MainGame/BluePrints/BP_FirstPersonCharacter` (`GameplayStatics.GetPlayerCharacter` 0)))
          (if (`self.IsAiming?_0`)
            (`|PlayMontage` null "/Game/_MainGame/Character/Animations/AimFire_Montage1.AimFire_Montage1"
              (:`then`
                _))
            (else
              (`|PlayMontage` null "/Game/_MainGame/Character/Animations/IdleFIre_Montage1.IdleFIre_Montage1"
                (:`then`
                  _))))
          (`SkeletalMeshComponent.PlayAnimation` (`self.AR`) null false)
          (bind (_outhit _returnvalue_3) (`KismetSystemLibrary.LineTraceSingle` _returnvalue_2 (+ _returnvalue_2 (* (`KismetMathLibrary.GetForwardVector` (`PlayerCameraManager.GetCameraRotation` _returnvalue)) (`self.WeaponRange_0`))) "TraceTypeQuery2" true (`|MakeArray` self :!type "Actor Object Reference") "Persistent"))
          (if _returnvalue_3
            (bind (_bblockinghit _binitialoverlap _time _distance _location _impactpoint _normal _impactnormal _physmat _hitactor) (`GameplayStatics.BreakHitResult` _outhit))
            (switch `EPhysicalSurface` (`PhysicalMaterial.SurfaceType` _physmat)
              (:`SurfaceType_Default`
                (if (`self.ActorHasTag` _hitactor "Zombie")
                  (`self.ApplyDamage` _hitactor _outhit 20.0 _returnvalue_2)
                  (`GameplayStatics.SpawnEmitterAtLocation` "/Game/Realistic_Starter_VFX_Pack_Vol2/Particles/Blood/P_Blood_Splat_Cone.P_Blood_Splat_Cone" _location :!label _label)
                  (else
                    (`GameplayStatics.SpawnEmitterAtLocation` "/Game/Realistic_Starter_VFX_Pack_Vol2/Particles/Hit/P_Asphalt.P_Asphalt" _location))))
              (:`SurfaceType1`
                (`self.ApplyDamage` _hitactor _outhit 50.0 _returnvalue_2)
                (goto _label))
              (:`SurfaceType2`
                (`self.ApplyDamage` _hitactor _outhit 20.0 _returnvalue_2)
                (goto _label)))))))))

(fn `Shoot_0`
  (params (isReloading :type Boolean) (magazine :type Integer))
  (returns (FirstPersonMesh :type "SkeletalMeshComponent Object Reference") (ReturnValue :type "Character Object Reference")))

(fn `UserConstructionScript`
  (`parent.UserConstructionScript`))