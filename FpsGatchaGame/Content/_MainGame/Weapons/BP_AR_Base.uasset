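; BP_AR_Base is a base assault rifle weapon with single and auto fire modes, clip and bag ammo, and delayed reloading.
; Firing line-traces from the player camera with persistent debug drawing and spends ammo; the Auto timeline repeats this shot at FireRateAuto.
; AmmoCheck updates the reload and empty-clip state for both firing and reloading.
; A Tick test simulates mesh physics until a zero-length trace reports a hit.
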(event `self.ReceiveTick`
  (params (DeltaSeconds :type "Float (single-precision)"))
  (bind _returnvalue (`self.K2_GetActorLocation`))
  (`|ExecutionSequence`
    (:`then_0`
      (if (`self.testFISICA`)
        (bind _outhit (`KismetSystemLibrary.LineTraceSingle` :`Start` _returnvalue :`End` (- _returnvalue (0.0 0.0 0.0)) :`TraceChannel` "TraceTypeQuery1" :`DrawDebugType` "ForDuration"))
        (if (`GameplayStatics.BreakHitResult` _outhit)
          (set `self.testFISICA` false)
          (`PrimitiveComponent.SetSimulatePhysics` (`self.SkeletalMesh`) false)
          (else
            (`PrimitiveComponent.SetSimulatePhysics` (`self.SkeletalMesh`) true)))))))

(event `Reload`
  (bind _ammoneeded (`self.AmmoNeeded`))
  ;[1 1 1] Reloading
  (`self.AmmoCheck`)
  (if (`self.CanReaload`)
    (set `self.Reloading` true)
    (`KismetSystemLibrary.Delay` (`self.ReloadDelay`))
    (if (`self.UseRemainingAmmo`)
      (set `self.ClipAmmo` (+ (`self.ClipAmmo`) (`self.BagAmmo`)))
      (set `self.BagAmmo` 0)
      (set `self.AmmoNeeded` 0)
      (set `self.Reloading` false)
      (else
        (set `self.ClipAmmo` (+ (`self.ClipAmmo`) _ammoneeded))
        (set `self.BagAmmo` (- (`self.BagAmmo`) _ammoneeded))
        (set `self.AmmoNeeded` 0)
        (set `self.Reloading` false)))))

(event `StartFire`
  (bind _returnvalue (`GameplayStatics.GetPlayerCameraManager` 0))
  (bind _returnvalue_2 (`PlayerCameraManager.GetCameraLocation` _returnvalue))
  ;[1 1 1] Firing
  (`TimelineComponent.SetTimelineLength` (`self.Auto`) (`self.FireRate_Auto`))
  (switch `/Game/_MainGame/Weapons/FireMode` (`self.Selection`)
    (:`NewEnumerator0`
      (`self.AmmoCheck` :!label _label)
      (if (`self.CanFire`)
        (if (not (`self.ClipEmpty`))
          (if (not (`self.Reloading`))
            (`KismetSystemLibrary.LineTraceSingle` _returnvalue_2 (+ _returnvalue_2 (* (`KismetMathLibrary.GetForwardVector` (`PlayerCameraManager.GetCameraRotation` _returnvalue)) (`self.WeaponRange`))) "TraceTypeQuery1" true (`|MakeArray` (stale `self.ReceiveBeginPlay` _asbp_first_person_character) self :!type "Actor Object Reference") "Persistent")
            (set `self.ClipAmmo` (- (`self.ClipAmmo`) (`self.AmmoCost`)))))))
    (:`NewEnumerator2`
      (`Timeline|Auto` :!label _label_2
        (:`Fire`
          (goto _label))))))

(event `StopFire`
  ;[1 1 1] Firing
  (`|ExecutionSequence`
    (:`then_0`
      (goto _label_2 :!via `SetNewTime`))
    (:`then_1`
      (goto _label_2 :!via `Stop`))))

(event `self.ReceiveBeginPlay`
  ;[1 1 1] Firing
  (bind _asbp_first_person_character (cast `/Game/_MainGame/BluePrints/BP_FirstPersonCharacter` (`GameplayStatics.GetPlayerCharacter` 0))))

(fn `AmmoCheck`
  (`|ExecutionSequence`
    (:`then_0`
      (set `self.AmmoNeeded` (- (`self.MaxClipAmmo`) (`self.ClipAmmo`))))
    (:`then_1`
      (if (<= (`self.AmmoNeeded`) (`self.BagAmmo`))
        (set `self.HasEnoughAmmo` true)
        (set `self.UseRemainingAmmo` false)
        (set `self.CanReaload` true)
        (elif (<= (`self.BagAmmo`) 0)
          (set `self.HasEnoughAmmo` false)
          (set `self.UseRemainingAmmo` false)
          (set `self.CanReaload` false)
          (else
            (set `self.HasEnoughAmmo` true)
            (set `self.UseRemainingAmmo` true)))))
    (:`then_2`
      (if (or (`self.HasEnoughAmmo`) (`self.UseRemainingAmmo`))
        (if (< (`self.ClipAmmo`) (`self.MaxBagAmmo`))
          (set `self.CanReaload` true)
          (else
            (set `self.CanReaload` false :!label _label)))
        (else
          (goto _label))))
    (:`then_3`
      (set `self.ClipEmpty` (<= (`self.ClipAmmo`) 0)))))

(fn `FireModeSwitch`
  (switch `/Game/_MainGame/Weapons/FireMode` (`self.Selection`)
    (:`NewEnumerator0`
      (set `self.Selection` "NewEnumerator2"))
    (:`NewEnumerator2`
      (set `self.Selection` "NewEnumerator0"))))

(fn `UserConstructionScript`
  (`parent.UserConstructionScript`))